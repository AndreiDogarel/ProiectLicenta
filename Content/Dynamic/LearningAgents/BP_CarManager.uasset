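; Car manager actor that sets up Learning Agents reinforcement learning to train or run a driving policy for learning vehicle pawns.
; BeginPlay has each pawn set its agent references, then builds the training environment, interactor, policy and critic from existing, non-reinitialized network assets.
; A shared-memory trainer process feeds a communicator for the PPO trainer.
; Each Tick runs either policy inference or training, chosen by the RunInference flag.
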(event EventBeginPlay
  (bind _shared_memory_settings (Variables|Default|GetShared%20Memory%20Settings))
  (Utilities|FlowControl|Sequence
    (:then_0
      (bind _outactors (Actor|GetAllActorsOfClass "/Game/Dynamic/LearningAgents/BP_LearningVehiclePawn.BP_LearningVehiclePawn_C"))
      (bind _output_get (Variables|Default|SetCarActors _outactors))
      (for _array_element _output_get
        (Default|SetAgentReferences _array_element)))
    (:then_1
      (bind _returnvalue (Class|LearningAgentsTrainingEnvironment|MakeTrainingEnvironment (Variables|Default|GetLearningAgentsManager) "/Game/Dynamic/LearningAgents/BP_RLTrainingEnvironment.BP_RLTrainingEnvironment_C" "TrainingEnvironment"))
      (Variables|Default|SetTrainingEnvironment _returnvalue))
    (:then_2
      (bind _returnvalue_2 (Class|LearningAgentsInteractor|MakeInteractor (Variables|Default|GetLearningAgentsManager) "/Game/Dynamic/LearningAgents/BP_RLInteractor.BP_RLInteractor_C" "Interactor"))
      (Variables|Default|SetInteractor _returnvalue_2))
    (:then_3
      (bind _returnvalue_3 (Class|LearningAgentsPolicy|MakePolicy (Variables|Default|GetLearningAgentsManager) (Variables|Default|GetInteractor) "/Script/LearningAgents.LearningAgentsPolicy" "Policy" "/Game/Dynamic/LearningAgents/DA_Encoder.DA_Encoder" "/Game/Dynamic/LearningAgents/DA_Policy.DA_Policy" "/Game/Dynamic/LearningAgents/DA_Decoder.DA_Decoder" false false false (Variables|Default|GetPolicy%20Settings) 1234))
      (Variables|Default|SetPolicy _returnvalue_3))
    (:then_4
      (bind _returnvalue_4 (Class|LearningAgentsCritic|MakeCritic (Variables|Default|GetLearningAgentsManager) (Variables|Default|GetInteractor) (Variables|Default|GetPolicy) "/Script/LearningAgents.LearningAgentsCritic" "Critic" "/Game/Dynamic/LearningAgents/DA_Critic.DA_Critic" false (Variables|Default|GetCritic%20Settings) 1234))
      (Variables|Default|SetCritic _returnvalue_4))
    (:then_5
      (bind _returnvalue_5 (Class|LearningAgentsCommunicatorLibrary|SpawnSharedMemoryTrainingProcess (Variables|Default|GetTrainer%20Process%20Settings) _shared_memory_settings))
      (bind _returnvalue_6 (Class|LearningAgentsCommunicatorLibrary|MakeSharedMemoryCommunicator _returnvalue_5 _shared_memory_settings))
      (Variables|Default|SetCommunicator _returnvalue_6))
    (:then_6
      (bind _returnvalue_7 (Class|LearningAgentsPPOTrainer|MakePPOTrainer (Variables|Default|GetLearningAgentsManager) (Variables|Default|GetInteractor) (Variables|Default|GetTrainingEnvironment) (Variables|Default|GetPolicy) (Variables|Default|GetCritic) (Variables|Default|GetCommunicator) "/Script/LearningAgentsTraining.LearningAgentsPPOTrainer" "PPOTrainer" (Variables|Default|GetTrainer%20Settings)))
      (Variables|Default|SetTrainer _returnvalue_7))))

(event EventTick
  (params (DeltaSeconds :type Float%20%28single-precision%29))
  (if (Variables|Default|GetRunInference)
    (Class|LearningAgentsPolicy|RunInference (Variables|Default|GetPolicy) 0.0)
    (else
      (Class|LearningAgentsPPOTrainer|RunTraining (Variables|Default|GetTrainer) (Variables|Default|GetTrainer%20Training%20Settings) (Variables|Default|GetTraining%20Game%20Settings) true true))))

(fn ConstructionScript)