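; Rocket League-style car pawn for Learning Agents, registering itself on BeginPlay with tagged LearningAgentsManager actors.
; Setter functions take throttle, steering, boost, jump and air-roll inputs, driving the vehicle movement component and rotating the mesh directly for air control.
; DoJump picks a ground jump, upside-down recovery, double jump or directional dash from the stored axes, using force impulses and timeline-driven flips.
; ResetFlags clears ball-hit, shot and goal flags.
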(event Custom|DoJump
  (params (IsJumping :type Boolean))
  (if IsJumping
    (if (Variables|Default|GetOnGround)
      (Audio|PlaySoundatLocation "/Game/Static/Sounds/RL_Jump_Cue.RL_Jump_Cue" (Transformation|GetWorldLocation (Variables|Character|GetMesh)) "0, 0, 0" 1.0 1.0 0.0 0 0 0 0)
      (Effects|SpawnEmitterAttached "/Game/Static/StarterContent/Particles/P_Explosion.P_Explosion" (Variables|Character|GetMesh) "None")
      (Physics|AddForce (Variables|Character|GetMesh) (* (Transformation|GetActorUpVector) "50000.000000,50000.000000,50000.000000") "None" true)
      (elif (Variables|Default|GetIsHeadOnGround)
        (Variables|Default|SetRotationOff true)
        (Variables|Default|SetIsDashable false)
        (Physics|AddForce (Variables|Character|GetMesh) (* (Transformation|GetActorUpVector) "-50000.000000,-50000.000000,-50000.000000") "None" true)
        (Utilities|FlowControl|FlipFlop
          (:A
            ;[0.05098 0.05098 0.05098] Head on Ground Logic
            (bind _timeinterval (Timeline|Agent_HeadToRight PlayFromStart)
              (:Update
                (Transformation|AddLocalRotation (Variables|Character|GetMesh) (Math|Rotator|MakeRotator (* (* _timeinterval 3.6e+02) (Utilities|Time|GetWorldDeltaSeconds)) 0.0 0.0) true true))
              (:Finished
                (Variables|Default|SetRotationOff true :!label _label))))
          (:B
            (bind _timeinterval_2 (Timeline|Agent_HeadToLeft PlayFromStart)
              (:Update
                (Transformation|AddLocalRotation (Variables|Character|GetMesh) (Math|Rotator|MakeRotator (* (* _timeinterval_2 -3.6e+02) (Utilities|Time|GetWorldDeltaSeconds)) 0.0 0.0) true true))
              (:Finished
                (goto _label)))))
        (else
          ;[0.05098 0.05098 0.05098] Dashing
          (if (Variables|Default|GetIsDashable)
            (Effects|SpawnEmitterAttached "/Game/Static/StarterContent/Particles/P_Explosion1.P_Explosion1" (Variables|Character|GetMesh) "None" "0.000000,0.000000,20.000000")
            (Variables|Default|SetRotationOff true)
            (Variables|Default|SetIsDashable false)
            (if (!= (Variables|Default|GetForwardAxis) 0.0)
              (Audio|PlaySoundatLocation "/Game/Static/Sounds/RL_Dash_Cue.RL_Dash_Cue" (Transformation|GetWorldLocation (Variables|Character|GetMesh)) "0, 0, 0" 1.0 1.0 0.0 0 0 0 0)
              (if (or (!= (Variables|Default|GetRightAxis) 0.0) (!= (Variables|Default|GetAirRollAxis) 0.0))
                (if (> (Variables|Default|GetForwardAxis) 0.0)
                  (if (or (> (Variables|Default|GetRightAxis) 0.0) (> (Variables|Default|GetAirRollAxis) 0.0))
                    (Physics|AddForce (Variables|Character|GetMesh) (* (Math|Vector|GetForwardVector (Variables|Default|GetCube)) "100000.000000,100000.000000,100000.000000") "None" true)
                    (Physics|AddForce (Variables|Character|GetMesh) (* (Math|Vector|GetRightVector (Variables|Default|GetCube)) "30000.000000,30000.000000,30000.000000") "None" true)
                    (bind _timeinterval_3 (Timeline|Agent_ForwardRight PlayFromStart)
                      (:Update
                        (Transformation|AddLocalRotation (Variables|Character|GetMesh) (Math|Rotator|MakeRotator (* (* (* _timeinterval_3 -2.6e+02) (Utilities|Time|GetWorldDeltaSeconds)) -1.0) (* (* _timeinterval_3 -2.6e+02) (Utilities|Time|GetWorldDeltaSeconds)) 0.0) true true))
                      (:Finished
                        (Variables|Default|SetRotationOff false :!label _label_2)))
                    (else
                      (Physics|AddForce (Variables|Character|GetMesh) (* (Math|Vector|GetForwardVector (Variables|Default|GetCube)) "100000.000000,100000.000000,100000.000000") "None" true)
                      (Physics|AddForce (Variables|Character|GetMesh) (* (Math|Vector|GetRightVector (Variables|Default|GetCube)) "-30000.000000,-30000.000000,-30000.000000") "None" true)
                      (bind _timeinterval_4 (Timeline|Agent_ForwardLeft PlayFromStart)
                        (:Update
                          (Transformation|AddLocalRotation (Variables|Character|GetMesh) (Math|Rotator|MakeRotator (* (* (* _timeinterval_4 -2.6e+02) (Utilities|Time|GetWorldDeltaSeconds)) 1.0) (* (* _timeinterval_4 -2.6e+02) (Utilities|Time|GetWorldDeltaSeconds)) 0.0) true true))
                        (:Finished
                          (goto _label_2)))))
                  (elif (or (> (Variables|Default|GetRightAxis) 0.0) (> (Variables|Default|GetAirRollAxis) 0.0))
                    (Physics|AddForce (Variables|Character|GetMesh) (* (Math|Vector|GetForwardVector (Variables|Default|GetCube)) "-100000.000000,-100000.000000,-100000.000000") "None" true)
                    (Physics|AddForce (Variables|Character|GetMesh) (* (Math|Vector|GetRightVector (Variables|Default|GetCube)) "30000.000000,30000.000000,30000.000000") "None" true)
                    (bind _timeinterval_5 (Timeline|Agent_BackwardRight PlayFromStart)
                      (:Update
                        (Transformation|AddLocalRotation (Variables|Character|GetMesh) (Math|Rotator|MakeRotator (* (* (* _timeinterval_5 2.6e+02) (Utilities|Time|GetWorldDeltaSeconds)) 1.0) (* (* _timeinterval_5 2.6e+02) (Utilities|Time|GetWorldDeltaSeconds)) 0.0) true true))
                      (:Finished
                        (goto _label_2)))
                    (else
                      (Physics|AddForce (Variables|Character|GetMesh) (* (Math|Vector|GetForwardVector (Variables|Default|GetCube)) "-100000.000000,-100000.000000,-100000.000000") "None" true)
                      (Physics|AddForce (Variables|Character|GetMesh) (* (Math|Vector|GetRightVector (Variables|Default|GetCube)) "-30000.000000,-30000.000000,-30000.000000") "None" true)
                      (bind _timeinterval_6 (Timeline|Agent_BackwardLeft PlayFromStart)
                        (:Update
                          (Transformation|AddLocalRotation (Variables|Character|GetMesh) (Math|Rotator|MakeRotator (* (* (* _timeinterval_6 2.6e+02) (Utilities|Time|GetWorldDeltaSeconds)) -1.0) (* (* _timeinterval_6 2.6e+02) (Utilities|Time|GetWorldDeltaSeconds)) 0.0) true true))
                        (:Finished
                          (goto _label_2))))))
                (elif (> (Variables|Default|GetForwardAxis) 0.0)
                  (Physics|AddForce (Variables|Character|GetMesh) (* (Math|Vector|GetForwardVector (Variables|Default|GetCube)) "100000.000000,100000.000000,100000.000000") "None" true)
                  (bind _timeinterval_7 (Timeline|Agent_Forward PlayFromStart)
                    (:Update
                      (Transformation|AddLocalRotation (Variables|Character|GetMesh) (Math|Rotator|MakeRotator 0.0 (* (* _timeinterval_7 -3.6e+02) (Utilities|Time|GetWorldDeltaSeconds)) 0.0) true true))
                    (:Finished
                      (goto _label_2)))
                  (else
                    (Physics|AddForce (Variables|Character|GetMesh) (* (Math|Vector|GetForwardVector (Variables|Default|GetCube)) "-100000.000000,-100000.000000,-100000.000000") "None" true)
                    (bind _timeinterval_8 (Timeline|Agent_Backward PlayFromStart)
                      (:Update
                        (Transformation|AddLocalRotation (Variables|Character|GetMesh) (Math|Rotator|MakeRotator 0.0 (* (* _timeinterval_8 3.6e+02) (Utilities|Time|GetWorldDeltaSeconds)) 0.0) true true))
                      (:Finished
                        (goto _label_2))))))
              (elif (or (!= (Variables|Default|GetRightAxis) 0.0) (!= (Variables|Default|GetAirRollAxis) 0.0))
                (Audio|PlaySoundatLocation "/Game/Static/Sounds/RL_DashSides_Cue.RL_DashSides_Cue" (Transformation|GetWorldLocation (Variables|Character|GetMesh)) "0, 0, 0" 1.0 1.0 0.0 0 0 0 0)
                (if (or (> (Variables|Default|GetRightAxis) 0.0) (> (Variables|Default|GetAirRollAxis) 0.0))
                  (Physics|AddForce (Variables|Character|GetMesh) (* (Math|Vector|GetRightVector (Variables|Default|GetCube)) "100000.000000,100000.000000,100000.000000") "None" true)
                  (bind _timeinterval_9 (Timeline|Agent_Right PlayFromStart)
                    (:Update
                      (Transformation|AddLocalRotation (Variables|Character|GetMesh) (Math|Rotator|MakeRotator (* (* _timeinterval_9 -3.6e+02) (Utilities|Time|GetWorldDeltaSeconds)) 0.0 0.0) true true))
                    (:Finished
                      (goto _label_2)))
                  (else
                    (Physics|AddForce (Variables|Character|GetMesh) (* (Math|Vector|GetRightVector (Variables|Default|GetCube)) "-100000.000000,-100000.000000,-100000.000000") "None" true)
                    (bind _timeinterval_10 (Timeline|Agent_Left PlayFromStart)
                      (:Update
                        (Transformation|AddLocalRotation (Variables|Character|GetMesh) (Math|Rotator|MakeRotator (* (* _timeinterval_10 3.6e+02) (Utilities|Time|GetWorldDeltaSeconds)) 0.0 0.0) true true))
                      (:Finished
                        (goto _label_2)))))
                (else
                  (Audio|PlaySoundatLocation "/Game/Static/Sounds/RL_DoubleJump_Cue.RL_DoubleJump_Cue" (Transformation|GetWorldLocation (Variables|Character|GetMesh)) "0, 0, 0" 1.0 1.0 0.0 0 0 0 0)
                  (Physics|AddForce (Variables|Character|GetMesh) (* (Transformation|GetActorUpVector) "50000.000000,50000.000000,50000.000000") "None" true)
                  (goto _label_2))))))))))

(event EventBeginPlay
  (|CallParentFunction)
  (bind _outactors (Actor|GetAllActorswithTag "LearningAgentsManager"))
  (for _array_element _outactors
    (Utilities|IsValid (Actor|GetComponentbyClass _array_element "/Script/LearningAgents.LearningAgentsManager")
      (:Is%20Valid
        (Class|LearningAgentsManager|AddAgent (Actor|GetComponentbyClass _array_element "/Script/LearningAgents.LearningAgentsManager") self)
        (Variables|Default|SetFoundManager true)))))

(fn ConstructionScript)

(fn SetThrottle
  (params (Input :type Float%20%28double-precision%29))
  (Variables|Default|SetForwardAxis Input)
  (if (Variables|Default|GetOnGround)
    (if (< (Variables|Default|GetSpeedKm) (Variables|Default|GetMaxNormalSpeed))
      (Class|ChaosVehicleMovementComponent|SetThrottleInput (Variables|Default|GetVehicleMovementComponent) (Variables|Default|GetForwardAxis) :!label _label))
    (else
      ;[0.05098 0.05098 0.05098] Setting up air control forward/backward
      (if (< (Variables|Default|GetForwardAxis) 0.0)
        (Transformation|AddLocalRotation (Variables|Character|GetMesh) (Math|Rotator|MakeRotator 0.0 (* (Utilities|Time|GetWorldDeltaSeconds) 3e+02) 0.0) true true)
        (goto _label)
        (elif (> (Variables|Default|GetForwardAxis) 0.0)
          (Transformation|AddLocalRotation (Variables|Character|GetMesh) (Math|Rotator|MakeRotator 0.0 (* (Utilities|Time|GetWorldDeltaSeconds) -3e+02) 0.0) true true)
          (goto _label))))))

(fn SetSteering
  (params (Input :type Float%20%28double-precision%29))
  (Variables|Default|SetRightAxis Input)
  (if (Variables|Default|GetOnGround)
    (Class|ChaosVehicleMovementComponent|SetSteeringInput (Variables|Default|GetVehicleMovementComponent) (* (Variables|Default|GetRightAxis) 5.0) :!label _label)
    (else
      ;[0.05098 0.05098 0.05098] Setting up air control left/right
      (if (< (Variables|Default|GetRightAxis) 0.0)
        (Transformation|AddLocalRotation (Variables|Character|GetMesh) (Math|Rotator|MakeRotator 0.0 0.0 (* (Utilities|Time|GetWorldDeltaSeconds) -3e+02)) true true)
        (goto _label)
        (elif (> (Variables|Default|GetRightAxis) 0.0)
          (Transformation|AddLocalRotation (Variables|Character|GetMesh) (Math|Rotator|MakeRotator 0.0 0.0 (* (Utilities|Time|GetWorldDeltaSeconds) 3e+02)) true true)
          (goto _label))))))

(fn SetBoosting
  (params (Input :type Boolean))
  (Variables|Default|SetIsBoosting Input)
  (if (> (Variables|Default|GetBoost) 0.0)
    (Utilities|FlowControl|Sequence
      (:then_0
        (Variables|Default|SetBoost (Math|Float|Clamp(Float) (- (Variables|Default|GetBoost) 0.6) 0.0 1e+02))
        (if (< (Variables|Default|GetSpeedKm) (Variables|Default|GetMaxBoostingSpeed))
          (Physics|AddForce (Variables|Character|GetMesh) (* (Transformation|GetActorForwardVector) "2500.000000,2500.000000,2500.000000") "None" true)))
      (:then_1
        (Utilities|FlowControl|DoOnce false
          (:Completed
            (Audio|SpawnSoundAttached "/Game/Static/Sounds/RL_Boosting_Cue.RL_Boosting_Cue" (Variables|Character|GetMesh) "None" "0, 0, 0" "0, 0, 0" "KeepRelativeOffset" false 1.0 1.0 0.0 0 0)))))))

(fn SetJumping
  (params (Input :type Boolean))
  (CallFunction|DoJump Input))

(fn SetAirRoll
  (params (Input :type Float%20%28double-precision%29))
  (Variables|Default|SetAirRollAxis Input)
  (if (not (Variables|Default|GetOnGround))
    ;[0.05098 0.05098 0.05098] Air roll direction
    (if (< (Variables|Default|GetAirRollAxis) 0.0)
      (Transformation|AddLocalRotation (Variables|Character|GetMesh) (Math|Rotator|MakeRotator (* (Utilities|Time|GetWorldDeltaSeconds) -3e+02) 0.0 0.0) true true)
      (elif (> (Variables|Default|GetAirRollAxis) 0.0)
        (Transformation|AddLocalRotation (Variables|Character|GetMesh) (Math|Rotator|MakeRotator (* (Utilities|Time|GetWorldDeltaSeconds) 3e+02) 0.0 0.0) true true)))))

(fn ResetFlags
  (Variables|Default|SetBallHit false)
  (Variables|Default|SetScoredGoal false)
  (Variables|Default|SetScoredOwnGoal false)
  (Variables|Default|SetShotOnTarget false))