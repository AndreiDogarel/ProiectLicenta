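; Learning Agents training environment that trains BP_LearningVehiclePawn agents with reinforcement learning to play car soccer.
; Rewards sum event bonuses for ball hits, goals, shots on target and saves, an own-goal penalty, and dense dot-product shaping from car velocity along DistanceToBall and ball velocity toward the enemy goal.
; Episodes terminate when the agent scores either goal type, and resets clear its flags and return it to its spawn point.
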(fn GatherAgentReward
  (params (AgentId :type Integer))
  (bind _returnvalue (Class|LearningAgentsManagerListener|GetAgent AgentId "/Game/Dynamic/LearningAgents/BP_LearningVehiclePawn.BP_LearningVehiclePawn_C"))
  (Utilities|IsValid _returnvalue
    (:Is%20Valid
      (Variables|Default|SetRewardActor _returnvalue)
      (return (+ (Class|LearningAgentsRewards|MakeRewardonCondition (Variables|/Game/Dynamic/VehicleTemplate/Blueprints/VehicleAdvPawn.VehicleAdvPawn_C|GetBallHit (Variables|Default|GetRewardActor)) 5.0 "ConditionReward" false 0) (Class|LearningAgentsRewards|MakeRewardonCondition (Variables|/Game/Dynamic/VehicleTemplate/Blueprints/VehicleAdvPawn.VehicleAdvPawn_C|GetScoredGoal (Variables|Default|GetRewardActor)) 1e+02 "ConditionReward" false 0) (Class|LearningAgentsRewards|MakeRewardonCondition (Variables|/Game/Dynamic/VehicleTemplate/Blueprints/VehicleAdvPawn.VehicleAdvPawn_C|GetScoredOwnGoal (Variables|Default|GetRewardActor)) -1e+02 "ConditionReward" false 0) (Class|LearningAgentsRewards|MakeReward (Math|Vector|DotProduct (Variables|/Game/Dynamic/VehicleTemplate/Blueprints/VehicleAdvPawn.VehicleAdvPawn_C|GetDistanceToBall (Variables|Default|GetRewardActor)) (Transformation|GetComponentVelocity (Variables|/Script/ChaosVehicles.WheeledVehiclePawn|GetMesh (Variables|Default|GetRewardActor)))) 0.05 "Reward" false 0) (Class|LearningAgentsRewards|MakeRewardonCondition (Variables|/Game/Dynamic/VehicleTemplate/Blueprints/VehicleAdvPawn.VehicleAdvPawn_C|GetShotOnTarget (Variables|Default|GetRewardActor)) 1e+01 "ConditionReward" false 0) (Class|LearningAgentsRewards|MakeReward (Math|Vector|DotProduct (Transformation|GetComponentVelocity (Variables|/Game/Dynamic/Blueprints/BP_Ball.BP_Ball_C|GetBall (Variables|/Game/Dynamic/VehicleTemplate/Blueprints/VehicleAdvPawn.VehicleAdvPawn_C|GetBall1 (Variables|Default|GetRewardActor)))) (Math|Vector|Normalize (- (Transformation|GetActorLocation (Variables|/Game/Dynamic/VehicleTemplate/Blueprints/VehicleAdvPawn.VehicleAdvPawn_C|GetEnemyGoal (Variables|Default|GetRewardActor))) (Transformation|GetWorldLocation (Variables|/Game/Dynamic/Blueprints/BP_Ball.BP_Ball_C|GetBall (Variables|/Game/Dynamic/VehicleTemplate/Blueprints/VehicleAdvPawn.VehicleAdvPawn_C|GetBall1 (Variables|Default|GetRewardActor))))))) 0.05 "Reward" false 0) (Class|LearningAgentsRewards|MakeRewardonCondition (Variables|/Game/Dynamic/VehicleTemplate/Blueprints/VehicleAdvPawn.VehicleAdvPawn_C|GetSavedGoal (Variables|Default|GetRewardActor)) 5e+01 "ConditionReward" false 0))))))

(fn GatherAgentCompletion
  (params (AgentId :type Integer))
  (bind _returnvalue (Class|LearningAgentsManagerListener|GetAgent AgentId "/Game/Dynamic/LearningAgents/BP_LearningVehiclePawn.BP_LearningVehiclePawn_C"))
  (Utilities|IsValid _returnvalue
    (:Is%20Valid
      (bind _output_get (Variables|Default|SetCompletionAgent _returnvalue))
      (if (Variables|/Game/Dynamic/VehicleTemplate/Blueprints/VehicleAdvPawn.VehicleAdvPawn_C|GetScoredGoal _output_get)
        (return "Termination")
        (elif (Variables|/Game/Dynamic/VehicleTemplate/Blueprints/VehicleAdvPawn.VehicleAdvPawn_C|GetScoredOwnGoal _output_get)
          (return "Termination"))))))

(fn ResetAgentEpisode
  (params (AgentId :type Integer))
  (bind _returnvalue (Class|LearningAgentsManagerListener|GetAgent AgentId "/Game/Dynamic/LearningAgents/BP_LearningVehiclePawn.BP_LearningVehiclePawn_C"))
  (Utilities|IsValid _returnvalue
    (:Is%20Valid
      (Default|ResetFlags _returnvalue)
      (Default|ResettoSpawnPoint _returnvalue))))