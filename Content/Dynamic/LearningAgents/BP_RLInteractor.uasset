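; Learning Agents interactor that lets reinforcement learning agents drive BP_LearningVehiclePawn cars in a car-soccer game.
; Observations combine velocity, boost, ground contact, world-axis offsets between car, ball and enemy goal, and a facing-to-goal dot product.
; Actions feed clamped throttle, steering, jump and air roll, plus boosting, into the pawn.
; Boost is specified as a float action but read with GetBoolAction, so the schema and reader disagree.
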(fn GatherAgentObservation
  (params (InObservationObject :type Learning%20Agents%20Observation%20Object%20Object%20Reference) (AgentId :type Integer))
  (Variables|Default|SetObsActor (Class|LearningAgentsManagerListener|GetAgent AgentId "/Game/Dynamic/LearningAgents/BP_LearningVehiclePawn.BP_LearningVehiclePawn_C"))
  (return (Class|LearningAgentsObservations|MakeStructObservation InObservationObject (Utilities|Map|MakeMap "Velocity" (Class|LearningAgentsObservations|MakeVelocityObservation InObservationObject (Transformation|GetVelocity (Variables|Default|GetObsActor)) (Transformation|GetActorTransform (Variables|Default|GetObsActor)) "VelocityObservation" false 0) "Boost" (Class|LearningAgentsObservations|MakeFloatObservation InObservationObject (Math|Float|NormalizetoRange (Variables|/Game/Dynamic/VehicleTemplate/Blueprints/VehicleAdvPawn.VehicleAdvPawn_C|GetBoost (Variables|Default|GetObsActor)) 0.0 1.0) "FloatObservation" false 0) "IsOnGround" (Class|LearningAgentsObservations|MakeFloatObservation InObservationObject (Math|Conversions|ToFloat(Boolean) (Variables|/Game/Dynamic/VehicleTemplate/Blueprints/VehicleAdvPawn.VehicleAdvPawn_C|GetOnGround (Variables|Default|GetObsActor))) "FloatObservation" false 0) "Ball-Agent" (Class|LearningAgentsObservations|MakeStructObservation InObservationObject (Utilities|Map|MakeMap "X" (Class|LearningAgentsObservations|MakeFloatObservation InObservationObject (.x (- (Transformation|GetActorLocation (Variables|Default|GetBallRef)) (Transformation|GetActorLocation (Variables|Default|GetObsActor)))) "FloatObservation" false 0) "Y" (Class|LearningAgentsObservations|MakeFloatObservation InObservationObject (.y (- (Transformation|GetActorLocation (Variables|Default|GetBallRef)) (Transformation|GetActorLocation (Variables|Default|GetObsActor)))) "FloatObservation" false 0) "Z" (Class|LearningAgentsObservations|MakeFloatObservation InObservationObject (.z (- (Transformation|GetActorLocation (Variables|Default|GetBallRef)) (Transformation|GetActorLocation (Variables|Default|GetObsActor)))) "FloatObservation" false 0))) "Goal-Agent" (Class|LearningAgentsObservations|MakeStructObservation InObservationObject (Utilities|Map|MakeMap "X" (Class|LearningAgentsObservations|MakeFloatObservation InObservationObject (.x (- (Transformation|GetActorLocation (Variables|/Game/Dynamic/VehicleTemplate/Blueprints/VehicleAdvPawn.VehicleAdvPawn_C|GetEnemyGoal (Variables|Default|GetObsActor))) (Transformation|GetActorLocation (Variables|Default|GetObsActor)))) "FloatObservation" false 0) "Y" (Class|LearningAgentsObservations|MakeFloatObservation InObservationObject (.y (- (Transformation|GetActorLocation (Variables|/Game/Dynamic/VehicleTemplate/Blueprints/VehicleAdvPawn.VehicleAdvPawn_C|GetEnemyGoal (Variables|Default|GetObsActor))) (Transformation|GetActorLocation (Variables|Default|GetObsActor)))) "FloatObservation" false 0) "Z" (Class|LearningAgentsObservations|MakeFloatObservation InObservationObject (.z (- (Transformation|GetActorLocation (Variables|/Game/Dynamic/VehicleTemplate/Blueprints/VehicleAdvPawn.VehicleAdvPawn_C|GetEnemyGoal (Variables|Default|GetObsActor))) (Transformation|GetActorLocation (Variables|Default|GetObsActor)))) "FloatObservation" false 0))) "Goal-Ball" (Class|LearningAgentsObservations|MakeStructObservation InObservationObject (Utilities|Map|MakeMap "X" (Class|LearningAgentsObservations|MakeFloatObservation InObservationObject (.x (- (Transformation|GetActorLocation (Variables|/Game/Dynamic/VehicleTemplate/Blueprints/VehicleAdvPawn.VehicleAdvPawn_C|GetEnemyGoal (Variables|Default|GetObsActor))) (Transformation|GetActorLocation (Variables|Default|GetBallRef)))) "FloatObservation" false 0) "Y" (Class|LearningAgentsObservations|MakeFloatObservation InObservationObject (.y (- (Transformation|GetActorLocation (Variables|/Game/Dynamic/VehicleTemplate/Blueprints/VehicleAdvPawn.VehicleAdvPawn_C|GetEnemyGoal (Variables|Default|GetObsActor))) (Transformation|GetActorLocation (Variables|Default|GetBallRef)))) "FloatObservation" false 0) "Z" (Class|LearningAgentsObservations|MakeFloatObservation InObservationObject (.z (- (Transformation|GetActorLocation (Variables|/Game/Dynamic/VehicleTemplate/Blueprints/VehicleAdvPawn.VehicleAdvPawn_C|GetEnemyGoal (Variables|Default|GetObsActor))) (Transformation|GetActorLocation (Variables|Default|GetBallRef)))) "FloatObservation" false 0))) "GoalAngle" (Class|LearningAgentsObservations|MakeFloatObservation InObservationObject (Math|Vector|DotProduct (Math|Vector|Normalize (- (Transformation|GetActorLocation (Variables|/Game/Dynamic/VehicleTemplate/Blueprints/VehicleAdvPawn.VehicleAdvPawn_C|GetEnemyGoal (Variables|Default|GetObsActor))) (Transformation|GetActorLocation (Variables|Default|GetObsActor)))) (Transformation|GetActorForwardVector (Variables|Default|GetObsActor))) "FloatObservation" false 0)))))

(fn SpecifyAgentObservation
  (params (InObservationSchema :type Learning%20Agents%20Observation%20Schema%20Object%20Reference))
  (return (Class|LearningAgentsObservations|SpecifyStructObservation InObservationSchema (Utilities|Map|MakeMap "Velocity" (Class|LearningAgentsObservations|SpecifyVelocityObservation InObservationSchema 2e+02) "Boost" (Class|LearningAgentsObservations|SpecifyFloatObservation InObservationSchema 1.0) "IsOnGround" (Class|LearningAgentsObservations|SpecifyFloatObservation InObservationSchema 1.0) "Ball-Agent" (Class|LearningAgentsObservations|SpecifyStructObservation InObservationSchema (Utilities|Map|MakeMap "X" (Class|LearningAgentsObservations|SpecifyFloatObservation InObservationSchema 1.0) "Y" (Class|LearningAgentsObservations|SpecifyFloatObservation InObservationSchema 1.0) "Z" (Class|LearningAgentsObservations|SpecifyFloatObservation InObservationSchema 1.0))) "Goal-Agent" (Class|LearningAgentsObservations|SpecifyStructObservation InObservationSchema (Utilities|Map|MakeMap "X" (Class|LearningAgentsObservations|SpecifyFloatObservation InObservationSchema 1.0) "Y" (Class|LearningAgentsObservations|SpecifyFloatObservation InObservationSchema 1.0) "Z" (Class|LearningAgentsObservations|SpecifyFloatObservation InObservationSchema 1.0))) "Goal-Ball" (Class|LearningAgentsObservations|SpecifyStructObservation InObservationSchema (Utilities|Map|MakeMap "X" (Class|LearningAgentsObservations|SpecifyFloatObservation InObservationSchema 1.0) "Y" (Class|LearningAgentsObservations|SpecifyFloatObservation InObservationSchema 1.0) "Z" (Class|LearningAgentsObservations|SpecifyFloatObservation InObservationSchema 1.0))) "GoalAngle" (Class|LearningAgentsObservations|SpecifyFloatObservation InObservationSchema 1.0)))))

(fn SpecifyAgentAction
  (params (InActionSchema :type Learning%20Agents%20Action%20Schema%20Object%20Reference))
  (return (Class|LearningAgentsActions|SpecifyStructAction InActionSchema (Utilities|Map|MakeMap "Throttle" (Class|LearningAgentsActions|SpecifyFloatAction InActionSchema 1.0) "Steering" (Class|LearningAgentsActions|SpecifyFloatAction InActionSchema 1.0) "Boost" (Class|LearningAgentsActions|SpecifyFloatAction InActionSchema 1.0) "Jump" (Class|LearningAgentsActions|SpecifyFloatAction InActionSchema 1.0) "AirRoll" (Class|LearningAgentsActions|SpecifyFloatAction InActionSchema 1.0)))))

(fn PerformAgentAction
  (params (InActionObject :type Learning%20Agents%20Action%20Object%20Object%20Reference) (InActionObjectElement :type Learning%20Agents%20Action%20Object%20Element%20Structure%20%28by%20ref%29) (AgentId :type Integer))
  (Variables|Default|SetActionActor (Class|LearningAgentsManagerListener|GetAgent AgentId "/Game/Dynamic/LearningAgents/BP_LearningVehiclePawn.BP_LearningVehiclePawn_C"))
  (bind _outelements (Class|LearningAgentsActions|GetStructAction InActionObject InActionObjectElement))
  (Utilities|FlowControl|Sequence
    (:then_0
      (bind _outvalue (Class|LearningAgentsActions|GetFloatAction InActionObject (.Value (Utilities|Map|Find _outelements "Throttle")) "FloatAction" false 0))
      (Default|SetThrottle (Variables|Default|GetActionActor) (Math|Float|Clamp(Float) _outvalue -1.0)))
    (:then_1
      (bind _outvalue_2 (Class|LearningAgentsActions|GetFloatAction InActionObject (.Value (Utilities|Map|Find _outelements "Steering")) "FloatAction" false 0))
      (Default|SetSteering (Variables|Default|GetActionActor) (Math|Float|Clamp(Float) _outvalue_2 -1.0)))
    (:then_2
      (bind _boutvalue (Class|LearningAgentsActions|GetBoolAction InActionObject (.Value (Utilities|Map|Find _outelements "Boost")) "BoolAction" false 0))
      (Default|SetBoosting (Variables|Default|GetActionActor) _boutvalue))
    (:then_3
      (bind _outvalue_3 (Class|LearningAgentsActions|GetFloatAction InActionObject (.Value (Utilities|Map|Find _outelements "Jump")) "FloatAction" false 0))
      (Default|SetJumping (Variables|Default|GetActionActor) (Math|Float|Clamp(Float) _outvalue_3 0.0)))
    (:then_4
      (bind _outvalue_4 (Class|LearningAgentsActions|GetFloatAction InActionObject (.Value (Utilities|Map|Find _outelements "AirRoll")) "FloatAction" false 0))
      (Default|SetAirRoll (Variables|Default|GetActionActor) (Math|Float|Clamp(Float) _outvalue_4 -1.0)))))