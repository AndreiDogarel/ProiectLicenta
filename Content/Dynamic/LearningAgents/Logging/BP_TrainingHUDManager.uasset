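; Manager Blueprint for an on-screen Learning Agents training log HUD in a car training setup.
; On BeginPlay it adds a WB_LearningAgentsLog widget to the viewport and stores the first BP_CarManager found as its training manager.
; Logic to push agent 0's episode step, reward and episode time into the widget exists but is disconnected, and Tick is empty, so the HUD never updates from here.
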(event EventBeginPlay
  (Utilities|FlowControl|Sequence
    (:then_0
      (bind _returnvalue (UserInterface|CreateWidget "/Game/Dynamic/LearningAgents/Logging/WB_LearningAgentsLog.WB_LearningAgentsLog_C"))
      (UserInterface|Viewport|AddtoViewport _returnvalue 0)
      (Variables|Default|SetAgentHUDRef _returnvalue))
    (:then_1
      (bind _outactors (Actor|GetAllActorsOfClass "/Game/Dynamic/LearningAgents/BP_CarManager.BP_CarManager_C"))
      (Variables|Default|SetTrainingManagerRef (Utilities|Array|Get(acopy) _outactors)))))

(event EventTick
  (params (DeltaSeconds :type Float%20%28single-precision%29)))

(fn ConstructionScript)