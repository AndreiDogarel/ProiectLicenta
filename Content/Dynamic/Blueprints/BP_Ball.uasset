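; Physics ball for a vehicle ball game, resettable to a stored position after a goal.
; Each tick, a downward trace that ignores vehicle pawns places two ground decals and a midpoint line, scaling one decal by height and showing the line only when high.
; Niagara trails run only at high speed.
; Hits from learning vehicle pawns flag that pawn and record it as last toucher.
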(event OnComponentHit(Ball)
  (params (HitComponent :type Primitive%20Component%20Object%20Reference) (OtherActor :type Actor%20Object%20Reference) (OtherComp :type Primitive%20Component%20Object%20Reference) (NormalImpulse :type Vector :default "0, 0, 0") (Hit :type Hit%20Result%20Structure%20%28by%20ref%29))
  ;[0.05098 0.05098 0.05098] Check collision with the actor
  (bind _asbp_learning_vehicle_pawn (Utilities|Casting|CastToBP_LearningVehiclePawn OtherActor))
  (Variables|/Game/Dynamic/LearningAgents/BP_LearningVehiclePawn.BP_LearningVehiclePawn_C|SetBallHit _asbp_learning_vehicle_pawn true)
  (Variables|Default|SetLastTouchedPawn _asbp_learning_vehicle_pawn))

(event Custom|ResetPosition
  ;[0.05098 0.05098 0.05098] Reset ball location when we score a goal
  (Physics|SetPhysicsLinearVelocity (Variables|Default|GetBall) "0, 0, 0" false "None")
  (Class|PrimitiveComponent|SetPhysicsAngularVelocityinDegrees (Variables|Default|GetBall) "0, 0, 0" false "None")
  (Transformation|SetWorldLocation (Variables|Default|GetBall) (Variables|Default|GetPosition) false false))

(event EventBeginPlay
  ;[0.05098 0.05098 0.05098] Add actors to ignore for the ball indicator decals
  (bind _outactors (Actor|GetAllActorsOfClass "/Game/Dynamic/VehicleTemplate/Blueprints/VehicleAdvPawn.VehicleAdvPawn_C"))
  (for _array_element _outactors
    (Utilities|Array|Add (Variables|Default|GetActorsToIgnore) _array_element)))

(event EventTick
  (params (DeltaSeconds :type Float%20%28single-precision%29))
  (bind _ball (Variables|Default|GetBall))
  (bind _returnvalue (Transformation|GetWorldLocation _ball))
  (bind (_x _y) (Math|Vector|BreakVector _returnvalue))
  (Utilities|FlowControl|Sequence
    (:then_0
      ;[0.15 0.15 0.15 0.5] Ball decals and line
      (bind (_outhit _returnvalue_2) (Collision|LineTraceByChannel _returnvalue (Math|Vector|MakeVector _x _y -3102.0) "TraceTypeQuery1" false (Variables|Default|GetActorsToIgnore) "None"))
      (if _returnvalue_2
        (Variables|Default|SetGroundLocation (.Location (Collision|BreakHitResult _outhit)))
        (Transformation|SetWorldLocation (Variables|Default|GetDecal1) (Variables|Default|GetGroundLocation) false false)
        (Transformation|SetWorldScale3D (Variables|Default|GetDecal2) (Math|Vector|MakeVector 0.1 (Math|Float|Clamp(Float) (/ 1e+02 (.Distance (Collision|BreakHitResult _outhit))) 0.0 0.6) (Math|Float|Clamp(Float) (/ 1e+02 (.Distance (Collision|BreakHitResult _outhit))) 0.0 0.6)))
        (if (> (.Distance (Collision|BreakHitResult _outhit)) 3e+02)
          (Rendering|SetVisibility (Variables|Default|GetLine) true false)
          (else
            (Rendering|SetVisibility (Variables|Default|GetLine) false false)))
        (Transformation|SetWorldLocation (Variables|Default|GetLine) (/ (+ (Variables|Default|GetGroundLocation) (Transformation|GetWorldLocation (Variables|Default|GetBall))) "2.000000,2.000000,2.000000") false false)))
    (:then_1
      ;[0.05098 0.05098 0.05098] Render particles based on speed
      (if (> (Math|Vector|VectorLength (Transformation|GetComponentVelocity (Variables|Default|GetBall))) 1.2e+03)
        (Components|Activation|Activate (Variables|Default|GetNiagara2) false)
        (else
          (Components|Activation|Deactivate (Variables|Default|GetNiagara3)))))))

(fn ConstructionScript)