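; Game mode for a timed two-team car-and-ball match, tracking score and returning to the main menu after announcing the winner or draw.
; BeginPlay creates the HUD, spawns the player and learning-vehicle bots at tagged target points using team and match type from GI_MainLevel.
; A self-looping one-second delay drives the countdown, while looping timers spawn boost orbs randomly within the spawn zone bounds.
; Reset returns vehicles and the ball to their starting positions.
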(event Custom|UpdateTime
  ;[0.05098 0.05098 0.05098] Update time event
  (if (Variables|Default|GetIsPlaying) :!label _label
    (if (<= (Variables|Default|GetTimeSeconds) 0)
      (if (<= (Variables|Default|GetTimeMinutes) 0)
        (Variables|Default|SetIsPlaying false)
        (bind _returnvalue (UserInterface|CreateWidget "/Game/Dynamic/UI/WinnerAnnouncer_UI.WinnerAnnouncer_UI_C"))
        (UserInterface|Viewport|AddtoViewport _returnvalue 0)
        (Input|SetInputModeUIOnly (Game|GetPlayerController 0) 0 "DoNotLock" false)
        (if (> (Variables|Default|GetBlueTeamScore) (Variables|Default|GetOrangeTeamScore))
          (Default|AnnounceWinner _returnvalue "Blue")
          (Default|ChangeTextColor _returnvalue "NewEnumerator0")
          (elif (== (Variables|Default|GetBlueTeamScore) (Variables|Default|GetOrangeTeamScore))
            (Default|AnnounceDraw _returnvalue)
            (else
              (Default|AnnounceWinner _returnvalue "Orange")
              (Default|ChangeTextColor _returnvalue "NewEnumerator1"))))
        (Utilities|FlowControl|Delay 2.0)
        (Game|OpenLevel(byName) "LVL_MainMenu")
        (else
          (bind _result (Math|Integer|DecrementInt (Variables|Default|GetTimeMinutes))
            (:%20%20
              (Variables|Default|SetTimeMinutes _result)
              (Variables|Default|SetTimeSeconds 59)
              (Default|UpdateHUDTime (Variables|Default|GetHUD_UI) :!label _label_2)
              (Utilities|FlowControl|Delay 1.0)
              (goto _label)))))
      (else
        (Variables|Default|SetTimeSeconds (- (Variables|Default|GetTimeSeconds) 1))
        (goto _label_2)))))

(event Custom|UpdateScore
  (params (ScoredTeam :type E_TeamType%20Enum :default "NewEnumerator0"))
  ;[0.05098 0.05098 0.05098] Update score event
  (if (Utilities|Enum|Equal(Enum) ScoredTeam "NewEnumerator0")
    (Math|Integer|IncrementInt (Variables|Default|GetBlueTeamScore)
      (:%20%20
        _))
    (else
      (Math|Integer|IncrementInt (Variables|Default|GetOrangeTeamScore)
        (:%20%20
          _))))
  (Default|UpdateHUDScore (Variables|Default|GetHUD_UI) ScoredTeam))

(event Custom|SpawnOrangeOrb
  (bind _spawnarea (Variables|Default|GetSpawnArea))
  (bind _cube (Variables|/Game/Dynamic/Blueprints/BP_SpawnZone.BP_SpawnZone_C|GetCube _spawnarea))
  (bind (_origin _boxextent) (Collision|GetComponentBounds _cube))
  (bind _returnvalue (- _origin _boxextent))
  (bind _returnvalue_2 (+ _origin _boxextent))
  ;[0.05098 0.05098 0.05098] Spawn a boost orb in a random point
  (Game|SpawnActorfromClass "/Game/Dynamic/Blueprints/BP_OrangeBoost.BP_OrangeBoost_C" (Math|Transform|MakeTransform (Math|Vector|MakeVector (Math|Random|RandomFloatinRange (.x _returnvalue) (.x _returnvalue_2)) (Math|Random|RandomFloatinRange (.y _returnvalue) (.y _returnvalue_2)) -2.9e+03)) "Undefined" "MultiplyWithRoot" 0 0))

(event Custom|SpawnBlueOrb
  (bind _spawnarea (Variables|Default|GetSpawnArea))
  (bind _cube (Variables|/Game/Dynamic/Blueprints/BP_SpawnZone.BP_SpawnZone_C|GetCube _spawnarea))
  (bind (_origin _boxextent) (Collision|GetComponentBounds _cube))
  (bind _returnvalue (- _origin _boxextent))
  (bind _returnvalue_2 (+ _origin _boxextent))
  ;[0.05098 0.05098 0.05098] Spawn a boost orb in a random point
  (Game|SpawnActorfromClass "/Game/Dynamic/Blueprints/BP_BlueBoost.BP_BlueBoost_C" (Math|Transform|MakeTransform (Math|Vector|MakeVector (Math|Random|RandomFloatinRange (.x _returnvalue) (.x _returnvalue_2)) (Math|Random|RandomFloatinRange (.y _returnvalue) (.y _returnvalue_2)) -2.9e+03)) "Undefined" "MultiplyWithRoot" 0 0))

(event Custom|SpawnOrangeOrbs
  ;[0.05098 0.05098 0.05098] Spawn a boost orb in a random point
  (CallFunction|SpawnOrangeOrb)
  (CallFunction|SpawnOrangeOrb)
  (CallFunction|SpawnOrangeOrb))

(event Custom|SpawnBlueOrbs
  ;[0.05098 0.05098 0.05098] Spawn a boost orb in a random point
  (CallFunction|SpawnBlueOrb)
  (CallFunction|SpawnBlueOrb)
  (CallFunction|SpawnBlueOrb))

(event EventBeginPlay
  (Utilities|FlowControl|Sequence
    (:then_0
      ;[0.05098 0.05098 0.05098] Set up HUD
      (bind _returnvalue (UserInterface|CreateWidget "/Game/Dynamic/UI/HUD_UI.HUD_UI_C" (Game|GetPlayerController 0)))
      (bind _output_get (Variables|Default|SetHUD_UI _returnvalue))
      (UserInterface|Viewport|AddtoViewport _output_get 0)
      (Utilities|FlowControl|Delay 1.0)
      (CallFunction|UpdateTime))
    (:then_1
      ;[0.05098 0.05098 0.05098] Set up the balls
      (bind _outactors (Actor|GetAllActorsOfClass "/Game/Dynamic/Blueprints/BP_Ball.BP_Ball_C"))
      (Variables|Default|SetBalls _outactors))
    (:then_2
      ;[0.05098 0.05098 0.05098] Set the spawn area
      (bind _outactors_2 (Actor|GetAllActorsOfClass "/Game/Dynamic/Blueprints/BP_SpawnZone.BP_SpawnZone_C"))
      (Variables|Default|SetSpawnArea (Utilities|Array|Get(acopy) _outactors_2)))
    (:then_3
      ;[0.05098 0.05098 0.05098] Set spawn timers for blue orbs
      (bind _returnvalue_2 (Utilities|Time|SetTimerbyFunctionName 0 "SpawnBlueOrbs" 2e+01 true false 1.0))
      (Variables|Default|SetSpawnBlueOrbsHandler _returnvalue_2))
    (:then_4
      ;[0.05098 0.05098 0.05098] Set spawn timers for orange orbs
      (bind _returnvalue_3 (Utilities|Time|SetTimerbyFunctionName 0 "SpawnOrangeOrbs" 2e+01 true false 1.0))
      (Variables|Default|SetSpawnOrangeOrbsHandler _returnvalue_3))
    (:then_5
      ;[0.05098 0.05098 0.05098] Set up spawn points for bots
      (bind _outactors_3 (Actor|GetAllActorsOfClasswithTag "/Script/Engine.TargetPoint" "SpawnBotOrange"))
      (Variables|Default|SetOrangeSpawnPoints _outactors_3))
    (:then_6
      (bind _outactors_4 (Actor|GetAllActorsOfClasswithTag "/Script/Engine.TargetPoint" "SpawnBotBlue"))
      (Variables|Default|SetBlueSpawnPoints _outactors_4))
    (:then_7
      ;[0.05098 0.05098 0.05098] Spawn player and bots
      (CallFunction|SpawnPlayer))
    (:then_8
      (CallFunction|SpawnBots))))

(fn ConstructionScript)

(fn Reset
  (bind _outactors (Actor|GetAllActorsOfClass "/Game/Dynamic/VehicleTemplate/Blueprints/VehicleAdvPawn.VehicleAdvPawn_C"))
  (for _array_element _outactors
    (Default|ResettoSpawnPoint _array_element))
  (Default|ResetPosition (Utilities|Array|Get(acopy) (Variables|Default|GetBalls))))

(fn SpawnPlayer
  (bind _returnvalue (Game|GetPlayerController 0))
  (bind _returnvalue_2 (Game|GetPlayerController 0))
  (bind _asgi_main_level (Utilities|Casting|CastToGI_MainLevel (Game|GetGameInstance)))
  (if (Utilities|Enum|Equal(Enum) (Variables|/Game/Dynamic/VehicleTemplate/Blueprints/GI_MainLevel.GI_MainLevel_C|GetSelectedTeam _asgi_main_level) "Blue")
    (bind _outactors (Actor|GetAllActorsOfClasswithTag "/Script/Engine.TargetPoint" "PlayerSpawnBlue"))
    (bind _returnvalue_3 (Game|SpawnActorfromClass "/Game/Dynamic/VehicleTemplate/Blueprints/SportsCar/SportsCar_Pawn.SportsCar_Pawn_C" (Math|Transform|MakeTransform (Transformation|GetActorLocation (Utilities|Array|Get(acopy) _outactors)) "0.000000,180.000000,0.000000") "Undefined" "MultiplyWithRoot" 0 "NewEnumerator0" (Transformation|GetActorLocation (Utilities|Array|Get(acopy) _outactors)) 0))
    (Pawn|Possess _returnvalue _returnvalue_3)
    (Default|SetAgentReferences _returnvalue_3)
    (Input|SetInputModeGameOnly _returnvalue false)
    (else
      (bind _outactors_2 (Actor|GetAllActorsOfClasswithTag "/Script/Engine.TargetPoint" "PlayerSpawnOrange"))
      (bind _returnvalue_4 (Game|SpawnActorfromClass "/Game/Dynamic/VehicleTemplate/Blueprints/SportsCar/SportsCar_Pawn.SportsCar_Pawn_C" (Math|Transform|MakeTransform (Transformation|GetActorLocation (Utilities|Array|Get(acopy) _outactors_2))) "Undefined" "MultiplyWithRoot" 0 "NewEnumerator1" (Transformation|GetActorLocation (Utilities|Array|Get(acopy) _outactors_2)) 0))
      (Pawn|Possess _returnvalue_2 _returnvalue_4)
      (Default|SetAgentReferences _returnvalue_4)
      (Input|SetInputModeGameOnly _returnvalue_2 false))))

(fn SpawnBots
  (bind _asgi_main_level (Utilities|Casting|CastToGI_MainLevel (Game|GetGameInstance)))
  (if (Utilities|Enum|Equal(Enum) (Variables|/Game/Dynamic/VehicleTemplate/Blueprints/GI_MainLevel.GI_MainLevel_C|GetSelectedTeam _asgi_main_level) "Blue")
    (Variables|Default|SetNumOfBlueBots (- (Math|Conversions|ToInteger(Byte) (.LeftS (Utilities|String|Split (Variables|/Game/Dynamic/VehicleTemplate/Blueprints/GI_MainLevel.GI_MainLevel_C|GetSelectedMatchType _asgi_main_level) "v"))) 1))
    (Variables|Default|SetNumOfOrangeBots (Math|Conversions|ToInteger(Byte) (.LeftS (Utilities|String|Split (Variables|/Game/Dynamic/VehicleTemplate/Blueprints/GI_MainLevel.GI_MainLevel_C|GetSelectedMatchType _asgi_main_level) "v"))))
    (else
      (Variables|Default|SetNumOfOrangeBots (- (Math|Conversions|ToInteger(Byte) (.RightS (Utilities|String|Split (Variables|/Game/Dynamic/VehicleTemplate/Blueprints/GI_MainLevel.GI_MainLevel_C|GetSelectedMatchType _asgi_main_level) "v"))) 1))
      (Variables|Default|SetNumOfBlueBots (Math|Conversions|ToInteger(Byte) (.RightS (Utilities|String|Split (Variables|/Game/Dynamic/VehicleTemplate/Blueprints/GI_MainLevel.GI_MainLevel_C|GetSelectedMatchType _asgi_main_level) "v"))))))
  (CallFunction|SpawnBlue)
  (CallFunction|SpawnOrange))

(fn SpawnBlue
  (for _index (range 0 (- (Variables|Default|GetNumOfBlueBots) 1))
    (Game|SpawnActorfromClass "/Game/Dynamic/LearningAgents/BP_LearningVehiclePawn.BP_LearningVehiclePawn_C" (Math|Transform|MakeTransform (Transformation|GetActorLocation (Utilities|Array|Get(acopy) (Variables|Default|GetBlueSpawnPoints) _index)) "0.000000,180.000000,0.000000") "Undefined" "MultiplyWithRoot" 0 "NewEnumerator0" (Transformation|GetActorLocation (Utilities|Array|Get(acopy) (Variables|Default|GetBlueSpawnPoints) _index)) 0)))

(fn SpawnOrange
  (for _index (range 0 (- (Variables|Default|GetNumOfOrangeBots) 1))
    (Game|SpawnActorfromClass "/Game/Dynamic/LearningAgents/BP_LearningVehiclePawn.BP_LearningVehiclePawn_C" (Math|Transform|MakeTransform (Transformation|GetActorLocation (Utilities|Array|Get(acopy) (Variables|Default|GetOrangeSpawnPoints) _index))) "Undefined" "MultiplyWithRoot" 0 "NewEnumerator1" (Transformation|GetActorLocation (Utilities|Array|Get(acopy) (Variables|Default|GetOrangeSpawnPoints) _index)) 0)))