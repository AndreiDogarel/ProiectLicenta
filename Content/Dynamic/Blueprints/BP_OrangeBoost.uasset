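; BP_OrangeBoost is a boost pickup that only vehicle pawns of one team, presumably orange, can collect.
; On sphere overlap, it checks the VehicleAdvPawn's Team enum, flags the boost as taken, sets Boost to a fixed full amount, calls UpdateBoost and destroys itself.
; An uncollected pickup destroys itself after a Lifetime delay started at BeginPlay.
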(event OnComponentBeginOverlap(SphereCollider)
  (params (OverlappedComponent :type Primitive%20Component%20Object%20Reference) (OtherActor :type Actor%20Object%20Reference) (OtherComp :type Primitive%20Component%20Object%20Reference) (OtherBodyIndex :type Integer) (bFromSweep :type Boolean) (SweepResult :type Hit%20Result%20Structure%20%28by%20ref%29))
  (bind _asvehicle_adv_pawn (Utilities|Casting|CastToVehicleAdvPawn OtherActor))
  (if (Utilities|Enum|Equal(Enum) (Variables|/Game/Dynamic/VehicleTemplate/Blueprints/VehicleAdvPawn.VehicleAdvPawn_C|GetTeam _asvehicle_adv_pawn) "NewEnumerator1")
    (Variables|/Game/Dynamic/VehicleTemplate/Blueprints/VehicleAdvPawn.VehicleAdvPawn_C|SetTookBoost _asvehicle_adv_pawn true)
    (Variables|/Game/Dynamic/VehicleTemplate/Blueprints/VehicleAdvPawn.VehicleAdvPawn_C|SetBoost _asvehicle_adv_pawn 1e+02)
    (Default|UpdateBoost _asvehicle_adv_pawn)
    (Actor|DestroyActor)))

(event EventBeginPlay
  (Utilities|FlowControl|Delay (Variables|Default|GetLifetime))
  (Actor|DestroyActor))

(fn ConstructionScript)